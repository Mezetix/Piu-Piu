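; Base Blueprint for a player-controlled thruster craft (Ladica) with guns and switchable first/third-person cameras.
; Setup calls configure guns, maneuver thrusters and hull, while movement, stepped throttle and fire inputs forward to functions defined outside these graphs.
; Aim axes orbit the camera in third person; pitch rotates the hull in first person, clamped by the thrusters' maximum rotation.
; Roll, yaw and Tick are empty, with older force and rotation logic left disconnected.
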(event `self.ReceiveBeginPlay`
  (`self.SetupManeverThrusters` (`self.ManeverTrusters`))
  (`self.SetupLadica` (`self.Ladica`)))

(event `self.ReceiveTick`
  (params (DeltaSeconds :type "Float (single-precision)")))

(event `InputAxis|AimHorizontal`
  (params (AxisValue :type "Float (single-precision)"))
  ;[1 1 1] Camera Look around
  (if (not (`self.1stPerson`))
    (`SceneComponent.K2_AddLocalRotation` (`self.AzimutRot`) (`KismetMathLibrary.MakeRotator` 0.0 0.0 AxisValue) false false)))

(event `InputAction|ThrustUpMax`
  (params (Key :type "Key Structure"))
  ;[1 1 1] Uravnava Gas - update u ticku
  (:`Released`
    (`self.ThrustMax`)))

(event `InputAxis|MoveUp`
  (params (AxisValue :type "Float (single-precision)"))
  ;[1 1 1] Bočno Premikanje
  (`self.MoveUpBase` AxisValue))

(event `InputAxis|AimVertical`
  (params (AxisValue :type "Float (single-precision)"))
  ;[1 1 1] Camera Look around
  (if (not (`self.1stPerson`))
    (`SceneComponent.K2_AddLocalRotation` (`self.SpringArm`) (`KismetMathLibrary.MakeRotator` 0.0 AxisValue) false false)))

(event `InputAction|ChangeCamera`
  (params (Key :type "Key Structure"))
  (bind _1stpersoncamera (`self.1stPersonCamera`))
  ;[1 1 1] Change Camera
  (:`Pressed`
    (`ActorComponent.ToggleActive` _1stpersoncamera)
    (`ActorComponent.ToggleActive` (`self.3rdPersonCamera`))
    (bind _output_get (set `self.1stPerson` (`ActorComponent.IsActive` _1stpersoncamera)))
    (if _output_get
      (`KismetSystemLibrary.PrintString` "1stPerson Camera active")
      (else
        (`KismetSystemLibrary.PrintString` "3rdPerson Camera active" true true (struct :`G` 1.0 :`B` 0.080762 :`A` 1.0))))))

(event `InputAxis|MoveRight`
  (params (AxisValue :type "Float (single-precision)"))
  ;[1 1 1] Bočno Premikanje
  (`self.MoveRightBase` AxisValue))

(event `InputAction|ThrustDownStop`
  (params (Key :type "Key Structure"))
  ;[1 1 1] Uravnava Gas - update u ticku
  (:`Released`
    (`self.ThrustStop`)))

(event `InputAxis|MoveFront`
  (params (AxisValue :type "Float (single-precision)"))
  ;[1 1 1] Bočno Premikanje
  (`self.MoveFrontBase` AxisValue))

(event `InputAction|ThrustUpOneStep`
  (params (Key :type "Key Structure"))
  ;[1 1 1] Uravnava Gas - update u ticku
  (:`Released`
    (`self.ThrustUpStep`)))

(event `InputAction|ThrustDownOneStep`
  (params (Key :type "Key Structure"))
  ;[1 1 1] Uravnava Gas - update u ticku
  (:`Released`
    (`self.ThrustDownStep`)))

(event `InputAction|FireGuns`
  (params (Key :type "Key Structure"))
  ;[1 1 1] Fire
  (:`Pressed`
    (`self.Fire`)))

(event `InputAxis|PitchUp`
  (params (AxisValue :type "Float (single-precision)"))
  ;[1 1 1] Roll pitch and Yaw .. in first person
  (bind _returnvalue (`ManeverTrusters.GetMaxSideRotation` (`self.ManeverTrusters`)))
  (if (`self.1stPerson`)
    (bind _returnvalue_2 (`KismetMathLibrary.Abs` _returnvalue))
    (`SceneComponent.K2_AddLocalRotation` (`self.Ladica`) (`KismetMathLibrary.MakeRotator` 0.0 (`KismetMathLibrary.FClamp` AxisValue (* _returnvalue_2 -1.0) _returnvalue_2)) false false)))

(event `InputAxis|RollRight`
  (params (AxisValue :type "Float (single-precision)"))
  ;[1 1 1] Roll pitch and Yaw .. in first person
)

(event `InputAxis|YawRight`
  (params (AxisValue :type "Float (single-precision)")))

(fn `GetNoramlisedRotYaw`
  (returns (RotationYaw :type "Float (double-precision)"))
  (bind _output_get (set `self.PlaneRotation` (.yaw (`SceneComponent.K2_GetComponentRotation` (`self.1stPersonCamera`)))))
  (if (>= _output_get 0.0)
    (return (`KismetMathLibrary.NormalizeToRange` (`self.PlaneRotation`) 0.0 360.0))
    (else
      (return (`KismetMathLibrary.NormalizeToRange` (`self.PlaneRotation`) 0.0 -360.0)))))

(fn `UserConstructionScript`
  (`self.SetupGuns` (`self.GunLeft`) (`self.GunRight`)))