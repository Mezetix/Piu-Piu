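; Projectile Blueprint that launches its physics-driven mesh in the direction it faces when play begins.
; BeginPlay sets ProjectileMesh's linear velocity to its world forward vector scaled by GetProjectileSpeed, replacing any existing velocity.
; An unconnected AddForce branch with a zero multiplier never runs, and the file has no overlap, tick or construction logic.
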(event `self.ReceiveBeginPlay`
  (bind _projectilemesh (`self.ProjectileMesh`))
  (bind _returnvalue (`self.GetProjectileSpeed`))
  (`PrimitiveComponent.SetPhysicsLinearVelocity` _projectilemesh (* (`KismetMathLibrary.Conv_RotatorToVector` (`SceneComponent.K2_GetComponentRotation` _projectilemesh)) _returnvalue) false "None"))

(event `self.ReceiveTick`
  (params (DeltaSeconds :type "Float (single-precision)")))

(fn `UserConstructionScript`)